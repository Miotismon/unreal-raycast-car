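; BP_Car is a drivable car Blueprint built from BP_CarWheelComponent children attached to the body mesh.
; The construction script copies the car's spring, raycast, rest distance and tire settings onto every wheel, suggesting raycast suspension handled inside those components.
; On BeginPlay it adds the Enhanced Input car mapping context.
; Steer input yaws steering wheels by input times a maximum angle, and release recenters all wheels.
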(event `EnhancedInput|/Game/Car/Input/IA_Steer`
  (params (ActionValue :type "Float (double-precision)") (ElapsedSeconds :type "Float (double-precision)") (TriggeredSeconds :type "Float (double-precision)") (InputAction :type "InputAction Object Reference" :default "/Game/Car/Input/IA_Steer.IA_Steer"))
  ; Steering
  (:`Triggered`
    (for _array_element (`SceneComponent.GetChildrenComponents` (`self.SM_CarBody`) false)
      (bind _asbp_car_wheel_component (cast `/Game/Car/BP_CarWheelComponent` _array_element))
      (if (`/Game/Car/BP_CarWheelComponent.IsSteering` _asbp_car_wheel_component)
        (`SceneComponent.K2_SetRelativeRotation` _asbp_car_wheel_component (`KismetMathLibrary.MakeRotator` 0.0 0.0 (* ActionValue (`self.MaxSteeringAngle`))) false false))))
  (:`Completed`
    (for _array_element_2 (`SceneComponent.GetChildrenComponents` (`self.SM_CarBody`) false)
      (bind _asbp_car_wheel_component_2 (cast `/Game/Car/BP_CarWheelComponent` _array_element_2))
      (`SceneComponent.K2_SetRelativeRotation` _asbp_car_wheel_component_2 (`KismetMathLibrary.MakeRotator` 0.0) false false))))

(event `self.ReceiveBeginPlay`
  (bind _returnvalue (`GameplayStatics.GetPlayerController` 0))
  (bind _returnvalue_2 (pcsubsystem `EnhancedInputLocalPlayerSubsystem` _returnvalue))
  (`/Engine/EditorBlueprintResources/StandardMacros.IsValid` _returnvalue
    (:`Is Valid`
      (`/Engine/EditorBlueprintResources/StandardMacros.IsValid` _returnvalue_2
        (:`Is Valid`
          (`EnhancedInputSubsystemInterface.AddMappingContext` _returnvalue_2 "/Game/Car/Input/IMC_Car.IMC_Car" 0 (struct)))
        (:`Is Not Valid`
          (`KismetSystemLibrary.PrintString` "uh oh 2"))))
    (:`Is Not Valid`
      (`KismetSystemLibrary.PrintString` "uhoh 0"))))

(event `self.ReceiveTick`
  (params (DeltaSeconds :type "Float (single-precision)")))

(fn `UserConstructionScript`
  (for _array_element (`SceneComponent.GetChildrenComponents` (`self.SM_CarBody`) false)
    (bind _asbp_car_wheel_component (cast `/Game/Car/BP_CarWheelComponent` _array_element))
    (set `/Game/Car/BP_CarWheelComponent.SpringStrength` (`self.SpringStrength`) _asbp_car_wheel_component)
    (set `/Game/Car/BP_CarWheelComponent.SpringDamping` (`self.SpringDamping`) _asbp_car_wheel_component)
    (set `/Game/Car/BP_CarWheelComponent.RayCastDistance` (`self.RayCastDistance`) _asbp_car_wheel_component)
    (set `/Game/Car/BP_CarWheelComponent.RestDistance` (`self.RestDistance`) _asbp_car_wheel_component)
    (set `/Game/Car/BP_CarWheelComponent.TireGripFactor` (`self.TireGripFactor`) _asbp_car_wheel_component)
    (set `/Game/Car/BP_CarWheelComponent.TireMass` (`self.TireMass`) _asbp_car_wheel_component)))