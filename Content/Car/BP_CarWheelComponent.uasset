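; Car wheel component that simulates raycast suspension and tire grip on a physics-driven static mesh parent.
; Each tick it traces down along its up vector; on a hit, it computes a damped spring force and a lateral anti-slip force from velocity at the wheel.
; Their sum is applied to the parent at the wheel's location.
; Acceleration and braking are unimplemented stubs.
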(event `self.ReceiveBeginPlay`)

(event `self.ReceiveTick`
  (params (DeltaSeconds :type "Float (single-precision)"))
  (bind (_raycasthitbool _raycasthitresult) (`self.RayCastToGround`))
  (if _raycasthitbool
    (bind _suspensionforce (`self.CalculateSuspensionForce` _raycasthitresult))
    (bind _steeringforce (`self.CalculateSteeringForce` DeltaSeconds))
    (`self.CalculateAccelerationForce`)
    ; apply force at spring location
    (bind _asstatic_mesh_component (cast `StaticMeshComponent` (`self.GetAttachParent`)))
    (`PrimitiveComponent.AddForceAtLocation` _asstatic_mesh_component (+ _steeringforce _suspensionforce) (`self.K2_GetComponentLocation`) "None")))

(fn `CalculateAccelerationForce`
  (returns (AccelerationForce :type "Vector Structure"))
  (return (0.0 0.0 0.0)))

(fn `CalculateBrakingForce`)

(fn `CalculateSteeringForce`
  (params (DeltaTime :type "Float (double-precision)"))
  (returns (SteeringForce :type "Vector Structure"))
  (bind _returnvalue (`self.GetRightVector`))
  (bind _asstatic_mesh_component (cast `StaticMeshComponent` (`self.GetAttachParent`)))
  (bind _returnvalue_2 (`PrimitiveComponent.GetPhysicsLinearVelocityAtPoint` _asstatic_mesh_component (`self.K2_GetComponentLocation`) "None"))
  (return (* (* (/ (* (* (`KismetMathLibrary.Dot_VectorVector` _returnvalue_2 _returnvalue) -1.0) (`self.TireGripFactor`)) DeltaTime) _returnvalue) (`self.TireMass`))))

(fn `CalculateSuspensionForce`
  (params (RayCastHitResult :type "HitResult Structure"))
  (returns (SuspensionForce :type "Vector Structure"))
  (bind _returnvalue (`self.GetUpVector`))
  (bind _asstatic_mesh_component (cast `StaticMeshComponent` (`self.GetAttachParent`)))
  (bind _returnvalue_2 (`PrimitiveComponent.GetPhysicsLinearVelocityAtPoint` _asstatic_mesh_component (`self.K2_GetComponentLocation`) "None"))
  (return (* (- (* (- (`self.RestDistance`) (`.Distance` (`GameplayStatics.BreakHitResult` RayCastHitResult))) (`self.SpringStrength`)) (* (`KismetMathLibrary.Dot_VectorVector` _returnvalue_2 _returnvalue) (`self.SpringDamping`))) _returnvalue)))

(fn `RayCastToGround`
  (returns (RayCastHitBool :type Boolean) (RayCastHitResult :type "HitResult Structure"))
  (bind _returnvalue (`self.K2_GetComponentLocation`))
  (bind (_outhit _returnvalue_2) (`KismetSystemLibrary.LineTraceSingle` :`Start` _returnvalue :`End` (- _returnvalue (* (`self.GetUpVector`) (`self.RayCastDistance`))) :`TraceChannel` "TraceTypeQuery1" :`DrawDebugType` "ForOneFrame"))
  (return _returnvalue_2 _outhit))