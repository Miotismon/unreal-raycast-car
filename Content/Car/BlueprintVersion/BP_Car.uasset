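; Player-driven car Blueprint that takes Enhanced Input for throttle, brake, steering and camera look.
; Construction copies shared suspension, grip, friction and mass tuning into each BP_CarWheelComponent under the body mesh.
; Steering yaws wheel components flagged as steering, while throttle and brake are only stored as variables here.
; Tick eases the spring arm toward the look target with frame-rate-independent smoothing and prints debug velocity.
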(event `EnhancedInput|/Game/Car/Input/IA_Camera`
  (params (ActionValue :type "Vector2D Structure") (ElapsedSeconds :type "Float (double-precision)") (TriggeredSeconds :type "Float (double-precision)") (InputAction :type "InputAction Object Reference" :default "/Game/Car/Input/IA_Camera.IA_Camera"))
  (bind (_x _y) (`KismetMathLibrary.BreakVector2D` ActionValue))
  (bind (_camerabaserotation_roll _camerabaserotation_pitch _camerabaserotation_yaw) (`KismetMathLibrary.BreakRotator` (`self.CameraBaseRotation`)))
  ; CameraTarget
  (:`Triggered`
    (set `self.CameraTargetRotation` (`KismetMathLibrary.MakeRotator` 0.0 (`KismetMathLibrary.Lerp` _camerabaserotation_pitch 30.0 _y) (`KismetMathLibrary.Lerp` _camerabaserotation_yaw 180.0 _x))))
  (:`Completed`
    (set `self.CameraTargetRotation` (`self.CameraBaseRotation`))))

(event `EnhancedInput|/Game/Car/Input/IA_Brake`
  (params (ActionValue :type "Float (double-precision)") (ElapsedSeconds :type "Float (double-precision)") (TriggeredSeconds :type "Float (double-precision)") (InputAction :type "InputAction Object Reference" :default "/Game/Car/Input/IA_Brake.IA_Brake"))
  ; Brake
  (:`Triggered`
    (set `self.InputBrake` ActionValue))
  (:`Completed`
    (set `self.InputBrake` 0.0)))

(event `EnhancedInput|/Game/Car/Input/IA_Throttle`
  (params (ActionValue :type "Float (double-precision)") (ElapsedSeconds :type "Float (double-precision)") (TriggeredSeconds :type "Float (double-precision)") (InputAction :type "InputAction Object Reference" :default "/Game/Car/Input/IA_Throttle.IA_Throttle"))
  ; Throttle
  (:`Triggered`
    (set `self.InputThrottle` ActionValue))
  (:`Completed`
    (set `self.InputThrottle` 0.0)))

(event `EnhancedInput|/Game/Car/Input/IA_Steer`
  (params (ActionValue :type "Float (double-precision)") (ElapsedSeconds :type "Float (double-precision)") (TriggeredSeconds :type "Float (double-precision)") (InputAction :type "InputAction Object Reference" :default "/Game/Car/Input/IA_Steer.IA_Steer"))
  ; Steering
  (:`Triggered`
    (for _array_element (`SceneComponent.GetChildrenComponents` (`self.SM_CarBody`) false)
      (bind _asbp_car_wheel_component (cast `/Game/Car/BlueprintVersion/BP_CarWheelComponent` _array_element))
      (if (`/Game/Car/BlueprintVersion/BP_CarWheelComponent.IsSteering` _asbp_car_wheel_component)
        (`SceneComponent.K2_SetRelativeRotation` _asbp_car_wheel_component (`KismetMathLibrary.MakeRotator` 0.0 0.0 (* ActionValue (`self.MaxSteeringAngle`))) false false))))
  (:`Completed`
    (for _array_element_2 (`SceneComponent.GetChildrenComponents` (`self.SM_CarBody`) false)
      (bind _asbp_car_wheel_component_2 (cast `/Game/Car/BlueprintVersion/BP_CarWheelComponent` _array_element_2))
      (`SceneComponent.K2_SetRelativeRotation` _asbp_car_wheel_component_2 (`KismetMathLibrary.MakeRotator` 0.0) false false))))

(event `self.ReceiveBeginPlay`
  (bind _returnvalue (`GameplayStatics.GetPlayerController` 0))
  (bind _returnvalue_2 (pcsubsystem `EnhancedInputLocalPlayerSubsystem` _returnvalue))
  ; Assign InputMappingContext on Start
  (`/Engine/EditorBlueprintResources/StandardMacros.IsValid` _returnvalue
    (:`Is Valid`
      (`/Engine/EditorBlueprintResources/StandardMacros.IsValid` _returnvalue_2
        (:`Is Valid`
          (`EnhancedInputSubsystemInterface.AddMappingContext` _returnvalue_2 "/Game/Car/Input/IMC_Car.IMC_Car" 0 (struct)))
        (:`Is Not Valid`
          (`KismetSystemLibrary.PrintString` "uh oh 2"))))
    (:`Is Not Valid`
      (`KismetSystemLibrary.PrintString` "uhoh 0"))))

(event `self.ReceiveTick`
  (params (DeltaSeconds :type "Float (single-precision)"))
  (bind _springarm (`self.SpringArm`))
  (`|ExecutionSequence`
    (:`then_0`
      ; Camera Smoothing
      (`SceneComponent.K2_SetRelativeRotation` _springarm (`KismetMathLibrary.RLerp` (`SceneComponent.RelativeRotation` _springarm) (`self.CameraTargetRotation`) (- 1.0 (`KismetMathLibrary.MultiplyMultiply_FloatFloat` (`self.CameraSmoothingRate`) DeltaSeconds))) false false))
    (:`then_1`
      ; Debug Text
      (bind _returnvalue (`PrimitiveComponent.GetPhysicsLinearVelocity` (`self.SM_CarBody`) "None"))
      (`KismetSystemLibrary.PrintText` (`|FormatText` "current velocity: {velocity}" (`KismetMathLibrary.VSize` _returnvalue)) true false (struct :`G` 0.66 :`B` 1.0 :`A` 1.0) 2.0 "Velocity"))))

(fn `UserConstructionScript`
  (set `self.CameraTargetRotation` (`self.CameraBaseRotation`))
  ; Setup Wheel Components
  (for _array_element (`SceneComponent.GetChildrenComponents` (`self.SM_CarBody`) false)
    (bind _asbp_car_wheel_component (cast `/Game/Car/BlueprintVersion/BP_CarWheelComponent` _array_element))
    (set `/Game/Car/BlueprintVersion/BP_CarWheelComponent.SpringStrength` (`self.SpringStrength`) _asbp_car_wheel_component)
    (set `/Game/Car/BlueprintVersion/BP_CarWheelComponent.SpringDamping` (`self.SpringDamping`) _asbp_car_wheel_component)
    (set `/Game/Car/BlueprintVersion/BP_CarWheelComponent.RayCastDistance` (`self.RayCastDistance`) _asbp_car_wheel_component)
    (set `/Game/Car/BlueprintVersion/BP_CarWheelComponent.RestDistance` (`self.RestDistance`) _asbp_car_wheel_component)
    (set `/Game/Car/BlueprintVersion/BP_CarWheelComponent.TireGripFactor` (`self.TireGripFactor`) _asbp_car_wheel_component)
    (set `/Game/Car/BlueprintVersion/BP_CarWheelComponent.RollingFrictionFactor` (`self.RollingFrictionFactor`) _asbp_car_wheel_component)
    (set `/Game/Car/BlueprintVersion/BP_CarWheelComponent.TireMass` (`self.TireMass`) _asbp_car_wheel_component)))