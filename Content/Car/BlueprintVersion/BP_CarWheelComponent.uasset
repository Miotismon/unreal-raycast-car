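; Scene component for one raycast wheel of BP_CarOld that simulates suspension, tire grip, drive and braking on the car body.
; Each tick a downward trace feeds a spring-damper, lateral grip with rolling friction, and optional drive and brake forces using the owner's inputs and power curve.
; The summed force is applied to the parent mesh at the wheel's location, with debug arrows per force.
; The child wheel mesh follows the contact distance and spins with forward velocity.
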(event `self.ReceiveBeginPlay`)

(event `self.ReceiveTick`
  (params (DeltaSeconds :type "Float (single-precision)"))
  (bind _returnvalue (`self.K2_GetComponentLocation`))
  (bind _returnvalue_2 (`self.K2_GetComponentLocation`))
  (bind _returnvalue_3 (`self.K2_GetComponentLocation`))
  (bind _returnvalue_4 (`self.K2_GetComponentLocation`))
  (bind (_raycasthitbool _raycasthitresult) (`self.RayCastToGround`))
  (if _raycasthitbool
    (bind _suspensionforce (`self.CalculateSuspensionForce` _raycasthitresult))
    (`KismetSystemLibrary.DrawDebugArrow` _returnvalue (+ _returnvalue (* _suspensionforce 0.01)) 1.0 (struct :`G` 0.143784 :`B` 1.0 :`A` 1.0))
    (bind _steeringforce (`self.CalculateGripForce` DeltaSeconds))
    (`KismetSystemLibrary.DrawDebugArrow` _returnvalue_2 (+ _returnvalue_2 (* _steeringforce 0.01)) 1.0 (struct :`R` 0.030027 :`G` 1.0 :`B` 0.001664 :`A` 1.0))
    (if (`self.IsDrive`)
      (bind _accelerationforce (`self.CalculateAccelerationForce` _raycasthitresult))
      (`KismetSystemLibrary.DrawDebugArrow` _returnvalue_3 (+ _returnvalue_3 (* _accelerationforce 0.01)) 1.0 (struct :`R` 1.0 :`G` 0.010174 :`A` 1.0)))
    (if (`self.IsBrake`)
      (bind _brakingforce (`self.CalculateBrakingForce` DeltaSeconds))
      (`KismetSystemLibrary.DrawDebugArrow` _returnvalue_4 (+ _returnvalue_4 (* _brakingforce 0.01)) 1.0 (struct :`R` 1.0 :`B` 0.912403 :`A` 1.0)))
    ; apply force at spring location
    (bind _asstatic_mesh_component (cast `StaticMeshComponent` (`self.GetAttachParent`)))
    (`PrimitiveComponent.AddForceAtLocation` _asstatic_mesh_component (+ _brakingforce (+ _accelerationforce (+ _steeringforce _suspensionforce))) (`self.K2_GetComponentLocation`) "None")
    (`self.MoveWheelToContact` _raycasthitresult)
    (`self.RotateWheel` DeltaSeconds)
    (else
      (`self.MoveWheelToMaxDistance`)
      (`self.RotateWheel` DeltaSeconds))))

(fn `CalculateAccelerationForce`
  (params (RayCastHitResult :type "HitResult Structure"))
  (returns (AccelerationForce :type "Vector Structure"))
  (bind _returnvalue (`self.GetAttachParent`))
  (bind _asstatic_mesh_component (cast `StaticMeshComponent` _returnvalue))
  (bind _returnvalue_2 (`PrimitiveComponent.GetPhysicsLinearVelocityAtPoint` _asstatic_mesh_component (`self.K2_GetComponentLocation`) "None"))
  (bind _asbp_car (cast `/Game/Car/BlueprintVersion/BP_CarOld` (`self.GetOwner`)))
  (bind _returnvalue_3 (`KismetMathLibrary.FClamp` (/ (`KismetMathLibrary.Abs` (`KismetMathLibrary.Dot_VectorVector` _returnvalue_2 (`self.GetForwardVector` _returnvalue))) (`/Game/Car/BlueprintVersion/BP_CarOld.TopSpeed` _asbp_car))))
  (if (>= _returnvalue_3 1.0)
    (return (0.0 0.0 0.0))
    (else
      (return (`KismetMathLibrary.ProjectVectorOnToPlane` (* (* (* (`CurveFloat.GetFloatValue` (`/Game/Car/BlueprintVersion/BP_CarOld.PowerCurve` _asbp_car) _returnvalue_3) (`/Game/Car/BlueprintVersion/BP_CarOld.MaxTorque` _asbp_car)) (`/Game/Car/BlueprintVersion/BP_CarOld.InputThrottle` _asbp_car)) (`self.GetForwardVector`)) (`.ImpactNormal` (`GameplayStatics.BreakHitResult` RayCastHitResult)))))))

(fn `CalculateBrakingForce`
  (params (DeltaTime :type "Float (double-precision)"))
  (returns (BrakingForce :type "Vector Structure"))
  (bind _returnvalue (`self.GetForwardVector`))
  (bind _asstatic_mesh_component (cast `StaticMeshComponent` (`self.GetAttachParent`)))
  (bind _returnvalue_2 (`PrimitiveComponent.GetPhysicsLinearVelocityAtPoint` _asstatic_mesh_component (`self.K2_GetComponentLocation`) "None"))
  (bind _asbp_car (cast `/Game/Car/BlueprintVersion/BP_CarOld` (`self.GetOwner`)))
  (bind _maxbreakingforce (`/Game/Car/BlueprintVersion/BP_CarOld.MaxBreakingForce` _asbp_car))
  (return (* (`KismetMathLibrary.FClamp` (* (/ (* (`/Game/Car/BlueprintVersion/BP_CarOld.InputBrake` _asbp_car) (* (`KismetMathLibrary.Dot_VectorVector` _returnvalue_2 _returnvalue) -1.0)) DeltaTime) (`/Game/Car/BlueprintVersion/BP_CarOld.BreakingStrength` _asbp_car)) (* _maxbreakingforce -1.0) _maxbreakingforce) _returnvalue)))

(fn `CalculateGripForce`
  (params (DeltaTime :type "Float (double-precision)"))
  (returns (SteeringForce :type "Vector Structure"))
  (bind _returnvalue (`self.GetRightVector`))
  (bind _returnvalue_2 (`self.GetForwardVector`))
  (bind _asstatic_mesh_component (cast `StaticMeshComponent` (`self.GetAttachParent`)))
  (bind _returnvalue_3 (`PrimitiveComponent.GetPhysicsLinearVelocityAtPoint` _asstatic_mesh_component (`self.K2_GetComponentLocation`) "None"))
  (bind _returnvalue_4 (`KismetMathLibrary.Dot_VectorVector` _returnvalue_3 _returnvalue_2))
  (if (>= (`KismetMathLibrary.Abs` _returnvalue_4) 1.0)
    (bind _returnvalue_5 (* (* (/ (* (* (`KismetMathLibrary.Dot_VectorVector` _returnvalue_3 _returnvalue) -1.0) (`self.TireGripFactor`)) DeltaTime) _returnvalue) (`self.TireMass`)))
    (return (+ (* (/ (* (* (`KismetMathLibrary.SignOfFloat` _returnvalue_4) -1.0) (`self.RollingFrictionFactor`)) DeltaTime) _returnvalue_2) _returnvalue_5))
    (else
      (return _returnvalue_5))))

(fn `CalculateSuspensionForce`
  (params (RayCastHitResult :type "HitResult Structure"))
  (returns (SuspensionForce :type "Vector Structure"))
  (bind _returnvalue (`self.GetUpVector`))
  (bind _asstatic_mesh_component (cast `StaticMeshComponent` (`self.GetAttachParent`)))
  (bind _returnvalue_2 (`PrimitiveComponent.GetPhysicsLinearVelocityAtPoint` _asstatic_mesh_component (`self.K2_GetComponentLocation`) "None"))
  (return (* (- (* (- (`self.RestDistance`) (`.Distance` (`GameplayStatics.BreakHitResult` RayCastHitResult))) (`self.SpringStrength`)) (* (`KismetMathLibrary.Dot_VectorVector` _returnvalue_2 _returnvalue) (`self.SpringDamping`))) _returnvalue)))

(fn `MoveWheelToContact`
  (params (RayCastHitResult :type "HitResult Structure"))
  (bind _asstatic_mesh_component (cast `StaticMeshComponent` (`self.GetChildComponent` 0)))
  (`self.K2_SetRelativeLocation` _asstatic_mesh_component (`KismetMathLibrary.MakeVector` 0.0 0.0 (* (- (`.Distance` (`GameplayStatics.BreakHitResult` RayCastHitResult)) (`self.WheelRadius`)) -1.0)) false false))

(fn `MoveWheelToMaxDistance`
  (bind _asstatic_mesh_component (cast `StaticMeshComponent` (`self.GetChildComponent` 0)))
  (`self.K2_SetRelativeLocation` _asstatic_mesh_component (`KismetMathLibrary.MakeVector` 0.0 0.0 (* (- (`self.RayCastDistance`) (`self.WheelRadius`)) -1.0)) false false))

(fn `RayCastToGround`
  (returns (RayCastHitBool :type Boolean) (RayCastHitResult :type "HitResult Structure"))
  (bind _returnvalue (`self.K2_GetComponentLocation`))
  (bind (_outhit _returnvalue_2) (`KismetSystemLibrary.LineTraceSingle` :`Start` _returnvalue :`End` (- _returnvalue (* (`self.GetUpVector`) (`self.RayCastDistance`))) :`TraceChannel` "TraceTypeQuery1" :`DrawDebugType` "ForOneFrame"))
  (return _returnvalue_2 _outhit))

(fn `RotateWheel`
  (params (DeltaTime :type "Float (double-precision)"))
  (bind _asstatic_mesh_component (cast `StaticMeshComponent` (`self.GetAttachParent`)))
  (bind _returnvalue (`PrimitiveComponent.GetPhysicsLinearVelocityAtPoint` _asstatic_mesh_component (`self.K2_GetComponentLocation`) "None"))
  (bind _asstatic_mesh_component_2 (cast `StaticMeshComponent` (`self.GetChildComponent` 0)))
  (`self.K2_AddLocalRotation` _asstatic_mesh_component_2 (`KismetMathLibrary.MakeRotator` 0.0 0.0 (* (`KismetMathLibrary.MultiplyByPi` (* (* (* (/ (`KismetMathLibrary.Dot_VectorVector` _returnvalue (`self.GetForwardVector`)) 100.0) 1.0) DeltaTime) 1.0)) (`self.WheelRadius`))) false false))