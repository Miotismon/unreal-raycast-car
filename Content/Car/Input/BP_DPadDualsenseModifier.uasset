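; An Enhanced Input modifier that turns the DualSense D-pad's raw analog reading into a 2D direction vector.
; ModifyRaw compares the input's X value to a raw-value-to-direction table within a small tolerance.
; The matched direction enum becomes an Axis2D value with unit components, covering diagonals and a neutral state, with up mapped to negative Y.
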(fn `ModifyRaw`
  (params (PlayerInput :type "EnhancedPlayerInput Object Reference") (CurrentValue :type "InputActionValue Structure") (DeltaTime :type "Float (single-precision)"))
  (returns (ReturnValue :type "InputActionValue Structure"))
  (for _array_element (`self.DPadRawToEnumArray`)
    (bind (_dpadrawvalue _dpaddualsensedirection) (break `/Game/Car/Input/ST_DPadRawToEnum` _array_element))
    (if (`KismetMathLibrary.NearlyEqual_FloatFloat` _dpadrawvalue (`EnhancedInputLibrary.BreakInputActionValue` CurrentValue) 0.02)
      (switch `/Game/Car/Input/E_DPadDualsenseDirections` _dpaddualsensedirection
        (:`NewEnumerator8`
          (return (`EnhancedInputLibrary.MakeInputActionValueOfType` 0.0 0.0 0.0 "Axis2D")))
        (:`NewEnumerator0`
          (return (`EnhancedInputLibrary.MakeInputActionValueOfType` -1.0 -1.0 0.0 "Axis2D")))
        (:`NewEnumerator1`
          (return (`EnhancedInputLibrary.MakeInputActionValueOfType` -1.0 0.0 0.0 "Axis2D")))
        (:`NewEnumerator2`
          (return (`EnhancedInputLibrary.MakeInputActionValueOfType` -1.0 1.0 0.0 "Axis2D")))
        (:`NewEnumerator3`
          (return (`EnhancedInputLibrary.MakeInputActionValueOfType` 0.0 1.0 0.0 "Axis2D")))
        (:`NewEnumerator4`
          (return (`EnhancedInputLibrary.MakeInputActionValueOfType` 1.0 1.0 0.0 "Axis2D")))
        (:`NewEnumerator5`
          (return (`EnhancedInputLibrary.MakeInputActionValueOfType` 1.0 0.0 0.0 "Axis2D")))
        (:`NewEnumerator6`
          (return (`EnhancedInputLibrary.MakeInputActionValueOfType` 1.0 -1.0 0.0 "Axis2D")))
        (:`NewEnumerator7`
          (return (`EnhancedInputLibrary.MakeInputActionValueOfType` 0.0 -1.0 0.0 "Axis2D")))))))