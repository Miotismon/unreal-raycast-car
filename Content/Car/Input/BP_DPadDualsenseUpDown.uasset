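; BP_DPadDualsenseUpDown is an input modifier in the car input setup that turns a raw DualSense D-pad value into a vertical 1D axis.
; It takes the parent modifier's X output and matches it, within a small tolerance, against a lookup array of raw values and direction enums.
; The matched direction becomes positive for up, negative for down, or zero for none.
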(fn `ModifyRaw`
  (params (PlayerInput :type "EnhancedPlayerInput Object Reference") (CurrentValue :type "InputActionValue Structure") (DeltaTime :type "Float (single-precision)"))
  (returns (ReturnValue :type "InputActionValue Structure"))
  (for _array_element (`self.DPadRawToEnumArray`)
    (bind (_dpadrawvalue _dpaddualsensedirection) (break `/Game/Car/Input/ST_DPadRawToEnum` _array_element))
    (if (`KismetMathLibrary.NearlyEqual_FloatFloat` _dpadrawvalue (`EnhancedInputLibrary.BreakInputActionValue` (`parent.ModifyRaw` PlayerInput CurrentValue DeltaTime)) 0.02)
      (switch `/Game/Car/Input/E_DPadDualsenseDirections` _dpaddualsensedirection
        (:`NewEnumerator8`
          (return (`EnhancedInputLibrary.MakeInputActionValueOfType` 0.0 0.0 0.0 "Axis1D")))
        (:`NewEnumerator3`
          (return (`EnhancedInputLibrary.MakeInputActionValueOfType` -1.0 0.0 0.0 "Axis1D")))
        (:`NewEnumerator7`
          (return (`EnhancedInputLibrary.MakeInputActionValueOfType` 1.0 0.0 0.0 "Axis1D")))))))